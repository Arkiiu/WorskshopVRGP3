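; BP_Affiche is a poster actor that shows the painting matching the current level.
; On BeginPlay it reads LevelIndex from the GI_TP game instance and hides the components that do not match, among Provence, Lavande and Paris paintings.
; The first three indices each leave one painting visible, while index 3 and any other value hide all three.
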(event `self.ReceiveBeginPlay`
  (bind _asgi_tp (cast `/Game/Game/Benji/GI_TP` (`GameplayStatics.GetGameInstance`)))
  ;[1 1 1] En fonction de l'index du niveau actuel il rend visible l'affiche à afficher et rendre invisible les affiches qui ne doivent pas être affiché
  (switch `int` (`/Game/Game/Benji/GI_TP.LevelIndex` _asgi_tp)
    (:`Default`
      (`SceneComponent.SetVisibility` (`self.Painting_Provence`) false false :!label _label)
      (`SceneComponent.SetVisibility` (`self.Painting_Lavande`) false false)
      (`SceneComponent.SetVisibility` (`self.Painting_Paris`) false false))
    (:`0`
      (`SceneComponent.SetVisibility` (`self.Painting_Lavande`) false false)
      (`SceneComponent.SetVisibility` (`self.Painting_Paris`) false false))
    (:`1`
      (`SceneComponent.SetVisibility` (`self.Painting_Provence`) false false)
      (`SceneComponent.SetVisibility` (`self.Painting_Paris`) false false))
    (:`2`
      (`SceneComponent.SetVisibility` (`self.Painting_Provence`) false false)
      (`SceneComponent.SetVisibility` (`self.Painting_Lavande`) false false))
    (:`3`
      (goto _label))))

(event `self.ReceiveTick`
  (params (DeltaSeconds :type "Float (single-precision)")))

(fn `UserConstructionScript`)