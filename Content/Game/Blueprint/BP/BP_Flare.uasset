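; Flare, a firefly that travels along the level's BP_Spline while facing the VR player and pulsing its light.
; After a startup delay it picks a speed by GameInstance level index, then Tick derives spline distance from game time while the GameMode allows movement.
; At the spline's end it halts, triggering next-level transition and desaturation on level index 3.
; It also orients attached painting meshes; mid-path pause logic is unwired.
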(event `BeginPlay`
  (`KismetSystemLibrary.Delay` 25.0 :!label _label) ; Le temps choisi pour ce node représente le temps que met flare à apparraître
  (bind _asvrgame_mode (cast `/Game/VRTemplate/Blueprints/VRGameMode` (`GameplayStatics.GetGameMode`)))
  (set `self.GameMode` _asvrgame_mode) ; Référence du Game Mode
  (bind _asvrpawn (cast `/Game/Game/Benji/VRPawn` (`GameplayStatics.GetPlayerPawn` 0)))
  (set `self.VRPawn` _asvrpawn) ; Référence du joueur
  (bind _returnvalue (`GameplayStatics.GetActorOfClass` "/Game/Game/Blueprint/BP/BP_Spline.BP_Spline_C"))
  (set `self.BP_Spline` _returnvalue) ; Référence Spline dans le niveau actuel
  (bind _asgi_tp (cast `/Game/Game/Benji/GI_TP` (`GameplayStatics.GetGameInstance`)))
  (set `self.GameInstance` _asgi_tp) ; Référence du GameInstance personnalisé
  (bind _returnvalue_2 (`GameplayStatics.GetCurrentLevelName` true))
  (set `self.LevelName` _returnvalue_2) ; Référence du nom du level actuel
  ;[0.2792 0.863 0.1447] Permet à la luciole de bouger
  (set `/Game/VRTemplate/Blueprints/VRGameMode.Ismoving` true (`self.GameMode`))
  ;[0.2792 0.863 0.1447] Vitesse choisie en fonction du niveau
  (switch `int` (`/Game/Game/Benji/GI_TP.LevelIndex` (`self.GameInstance`)) ; En fonction de l'index du niveau actuel il effectue les tâche correspondantes
    (:`Default`
      (bind _output_get (set `self.OriginSpeed` 500.0))
      (set `self.Speed` _output_get))
    (:`0`
      (bind _output_get_2 (set `self.OriginSpeed` 100.0)) ; Ce node représente la vitesse d'origine, il a pour but de servir au moment où la luciole s'arrête, accélère, ralentis
      (set `self.Speed` _output_get_2))
    (:`1`
      (bind _output_get_3 (set `self.OriginSpeed` 100.0))
      (set `self.Speed` _output_get_3))
    (:`2`
      (bind _output_get_4 (set `self.OriginSpeed` 200.0))
      (set `self.Speed` _output_get_4))
    (:`3`
      (bind _output_get_5 (set `self.OriginSpeed` 50.0))
      (set `self.Speed` _output_get_5)))
  (`self.FlareLumiere`) ; Lance l'animation de la lumire de Flare qui boucle
)

(event `self.ReceiveBeginPlay`
  (goto _label))

(event `self.ReceiveTick`
  (params (DeltaSeconds :type "Float (single-precision)"))
  (bind _returnvalue (`SceneComponent.K2_GetComponentLocation` (`self.Sphere`)))
  (bind _returnvalue_2 (- _returnvalue (`SceneComponent.K2_GetComponentLocation` (`self.Cube`))))
  (`|ExecutionSequence`
    (:`then_0`
      (`|ExecutionSequence`
        (:`then_0`
          (bind _gamemode (`self.GameMode`)
            (:`then`
              (if (`/Game/VRTemplate/Blueprints/VRGameMode.Ismoving` _gamemode)
                ;[1 1 1] Vérification de la fin de boucle
                (if (`self.IsLoopEnd`)
                  (if (== (`/Game/Game/Benji/GI_TP.LevelIndex` (`self.GameInstance`)) 3)
                    (`self.EndLevelTransition`) ; Appel du custom Event "EndLevelTranstion"
                    (else
                      (`ActorComponent.Activate` (`self.Audio`) false)))
                  (set `/Game/VRTemplate/Blueprints/VRGameMode.Ismoving` false (`self.GameMode`))
                  (else
                    (`self.Deplacement`) ; Appel la fonction de déplacement
                  ))
                (else
                  (set `self.ConteurTemps` (`GameplayStatics.GetTimeSeconds`)) ; Permet de recalculer le temps du jeu pour que la luciole puisse être situé au bon endroit sur la spline
                )))
            (:`else`)))
        (:`then_1`
          ;[1 0.5776 0.06663] Calcul rotation affiche
          (`SceneComponent.K2_SetWorldLocationAndRotation` (`self.Painting_next_level`) (+ _returnvalue (* (`KismetMathLibrary.Normal` _returnvalue_2) -10.0)) (`KismetMathLibrary.MakeRotFromZY` _returnvalue_2 (`SceneComponent.GetForwardVector` (`self.Sphere`))) false false))))
    (:`then_1`
      ;[1 0.5776 0.06663] Rotation de l'affiche
      (`SceneComponent.K2_SetWorldRotation` (`self.Plane`) (`KismetMathLibrary.MakeRotFromZX` (- (`SceneComponent.K2_GetComponentLocation` (`/Game/Game/Benji/VRPawn.Camera` (`self.VRPawn`))) (`SceneComponent.K2_GetComponentLocation` (`self.Sphere`))) (0.0 0.0 1.0)) false false))))

(event `FlareLumiere`
  ;[1 0.5776 0.06663] Animation de la lumière
  (bind (_direction _newtrack_1) (`Timeline|LumièreLuciole` :!label _label_2)
    (:`Update`
      (`LightComponent.SetIntensity` (`self.PointLight`) (* (+ _newtrack_1 0.1) 100.0)))
    (:`Finished`
      (`KismetSystemLibrary.Delay` (`KismetMathLibrary.RandomFloatInRange` 0.0 1.0))
      (`/Engine/EditorBlueprintResources/StandardMacros.FlipFlop`
        (:`A`
          (goto _label_2 :!via `Reverse`))
        (:`B`
          (goto _label_2))))))

(event `EndLevelTransition`
  ;[1 0.3611 0.3644] Transition de fin et retour au début
  (`/Game/Game/Benji/VRPawn.NextLevel` (`self.VRPawn`))
  (`KismetMaterialLibrary.SetScalarParameterValue` "/Game/Game/Material/MPC/MPC_NoirBlanc.MPC_NoirBlanc" "Desaturation" 1.0))

(fn `ChangementLevel`
  (bind _levelnamelist (`/Game/Game/Benji/GI_TP.LevelNameList` (`self.GameInstance`)))
  (`/Engine/EditorBlueprintResources/StandardMacros.DoOnce` false :!label _label
    (:`Completed`
      (bind _returnvalue (`GameplayStatics.GetCurrentLevelName` true))
      (`GameplayStatics.OpenLevel` (`KismetStringLibrary.Conv_StringToName` (`|GetArrayItem` _levelnamelist (+ (`KismetArrayLibrary.Array_Find` _levelnamelist _returnvalue) 1))))
      (goto _label :!via `Reset`))))

(fn `Deplacement`
  (bind _sphere (`self.Sphere`))
  (bind _spline (`/Game/Game/Blueprint/BP/BP_Spline.Spline` (`self.BP_Spline`)))
  (bind _returnvalue (`SplineComponent.GetSplineLength` _spline))
  (bind _returnvalue_2 (mod (* (- (`GameplayStatics.GetTimeSeconds`) (`self.ConteurTemps`)) (`self.Speed`)) _returnvalue))
  (set `self.IsLoopEnd` (>= _returnvalue_2 (- _returnvalue 10.0)))
  ;[1 1 1] Regarde vers le joueur
  (`SceneComponent.K2_SetWorldRotation` _sphere (`KismetMathLibrary.FindLookAtRotation` (`SceneComponent.K2_GetComponentLocation` _sphere) (`SceneComponent.K2_GetComponentLocation` (`/Game/Game/Benji/VRPawn.Camera` (`self.VRPawn`)))) false false)
  (`SceneComponent.K2_SetWorldLocation` (`self.Sphere`) (`SplineComponent.GetLocationAtDistanceAlongSpline` _spline _returnvalue_2 "World") false false))

(fn `Stop Move`
  (set `self.Speed` 0.0)
  (`ActorComponent.Activate` (`self.Audio`) false))

(fn `TestPosition`
  (params (DiviseurDistance :type "Float (double-precision)") (MargeErreur :type "Float (double-precision)"))
  (returns (Bool :type Boolean))
  (bind _spline (`/Game/Game/Blueprint/BP/BP_Spline.Spline` (`self.BP_Spline`)))
  (return (and (== (`SplineComponent.GetLocationAtDistanceAlongSpline` _spline (/ (`SplineComponent.GetSplineLength` _spline) DiviseurDistance) "World") (`SceneComponent.K2_GetComponentLocation` (`self.Sphere`)) :`ErrorTolerance` MargeErreur) (not (`self.IsAlreadyPause`)))))

(fn `UserConstructionScript`)