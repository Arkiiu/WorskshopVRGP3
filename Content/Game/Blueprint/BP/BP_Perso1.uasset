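; BP_Perso1 is a character Blueprint whose two eye lights pulse in brightness, starting at BeginPlay.
; The BrillanceYeux timeline drives the intensity of EyeRight and EyeRight1 together, scaled and clamped.
; Each time it finishes, a short random delay feeds a FlipFlop that alternates Reverse and Play, looping the glow at irregular intervals.
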(event `self.ReceiveBeginPlay`
  (`self.AnimYeux`))

(event `AnimYeux`
  ;[1 0.5776 0.06663] Animation de l'affiche qui flotte
  (bind (_direction _newtrack_0) (`Timeline|BrillanceYeux` :!label _label)
    (:`Update`
      (bind _returnvalue (`KismetMathLibrary.FClamp` (* _newtrack_0 500.0) 0.0 100.0))
      (`LightComponent.SetIntensity` (`self.EyeRight1`) _returnvalue)
      (`LightComponent.SetIntensity` (`self.EyeRight`) _returnvalue))
    (:`Finished`
      (`KismetSystemLibrary.Delay` (`KismetMathLibrary.RandomFloatInRange` 1.0 3.0))
      (`/Engine/EditorBlueprintResources/StandardMacros.FlipFlop`
        (:`A`
          (goto _label :!via `Reverse`))
        (:`B`
          (goto _label))))))

(fn `UserConstructionScript`)