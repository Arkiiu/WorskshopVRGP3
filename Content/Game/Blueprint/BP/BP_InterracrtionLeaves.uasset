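; BP_InterracrtionLeaves is an interactive leaves actor that plays audio when another actor overlaps it.
; On BeginPlay it casts the first player pawn to VRPawn and caches it.
; On overlap, a NOR check against the pawn's right and left hands activates the Audio component without reset only when the other actor is neither hand.
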(event `self.ReceiveBeginPlay`
  (bind _asvrpawn (cast `/Game/Game/Benji/VRPawn` (`GameplayStatics.GetPlayerPawn` 0)))
  (set `self.As VRPawn` _asvrpawn))

(event `self.ReceiveActorBeginOverlap`
  (params (OtherActor :type "Actor Object Reference"))
  (bind _as_vrpawn (`self.As VRPawn`))
  (if (`KismetMathLibrary.BooleanNOR` (== (`/Game/Game/Benji/VRPawn.HandR` _as_vrpawn) OtherActor) (== OtherActor (`/Game/Game/Benji/VRPawn.HandL` _as_vrpawn)))
    (`ActorComponent.Activate` (`self.Audio`) false)))

(fn `UserConstructionScript`)