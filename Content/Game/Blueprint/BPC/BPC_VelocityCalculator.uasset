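; BPC_VelocityCalculator is a component that measures its own world-space velocity from frame-to-frame movement.
; Each Tick, it derives an exact velocity from the change in world location since the previous frame divided by delta time.
; It then lerps an average velocity toward that value, scaled by delta time and a coefficient, to smooth out jitter, and stores the current location for the next frame.
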(event `self.ReceiveTick`
  (params (DeltaSeconds :type "Float (single-precision)"))
  (`|ExecutionSequence`
    (:`then_0`
      (set `self.ExactVelocity` (/ (- (`self.K2_GetComponentLocation`) (`self.PreviousLocation`)) DeltaSeconds)))
    (:`then_1`
      (set `self.AverageVelocity` (`KismetMathLibrary.VLerp` (`self.AverageVelocity`) (`self.ExactVelocity`) (* DeltaSeconds (`self.lerpCoef`)))))
    (:`then_2`
      ;[1 1 1] Mise à jour de la prévious location
      (set `self.PreviousLocation` (`self.K2_GetComponentLocation`)))))