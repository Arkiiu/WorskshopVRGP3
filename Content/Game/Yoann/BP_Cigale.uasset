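; BP_Cigale is an actor whose sphere travels point to point around the BP_Spline found in the level at BeginPlay.
; Each tick eases the sphere toward the current spline point with a delta-scaled lerp, adding the spline's world location to the already world-space point position.
; When close, it advances the index with wraparound and prints debug values.
; An unconnected closest-point follow snippet and an empty Deplacement function remain unused.
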(event `self.ReceiveBeginPlay`
  (bind _returnvalue (`GameplayStatics.GetActorOfClass` "/Game/Game/Yoann/BP_Spline.BP_Spline_C"))
  (set `self.BP_Spline` _returnvalue))

(event `self.ReceiveTick`
  (params (DeltaSeconds :type "Float (single-precision)"))
  (bind _spline (`/Game/Game/Yoann/BP_Spline.Spline` (`self.BP_Spline`)))
  (bind (_returnvalue_inputkey _returnvalue_position) (break `SplinePoint` (`SplineComponent.GetSplinePointAt` _spline (`self.PointIndex`) "World")))
  (bind _returnvalue (+ _returnvalue_position (`SceneComponent.K2_GetComponentLocation` _spline)))
  ;[1 1 1] Calcul de la position de la sphère
  (`SceneComponent.K2_SetWorldLocation` (`self.Sphere`) (`KismetMathLibrary.VLerp` (`SceneComponent.K2_GetComponentLocation` (`self.Sphere`)) _returnvalue (* DeltaSeconds 5.0)) false true)
  (if (< (`KismetMathLibrary.Vector_Distance` _returnvalue (`SceneComponent.K2_GetComponentLocation` (`self.Sphere`))) 10.0)
    (bind _output_get (set `self.PointIndex` (mod (+ (`self.PointIndex`) 1) (`SplineComponent.GetNumberOfSplinePoints` (`/Game/Game/Yoann/BP_Spline.Spline` (`self.BP_Spline`))))))
    (`KismetSystemLibrary.PrintString` (`KismetStringLibrary.Conv_IntToString` _output_get))
    (`KismetSystemLibrary.PrintString` (`KismetStringLibrary.Conv_BoolToString` (`SceneComponent.bVisible` (`self.Sphere`))))))

(fn `Deplacement`)

(fn `UserConstructionScript`)