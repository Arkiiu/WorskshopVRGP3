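; BP_Perso1 is a guide character (a firefly or cicada, per comments) whose Plane follows the BP_SplinePerso spline.
; Position derives from elapsed time times speed, wrapped by spline length, with ConteurTemps offsetting the clock.
; In three named levels it pauses two seconds at mid-spline, re-armed each loop; LevelFinal stops at loop end.
; Setup of LevelName, speed and IsMoving is disconnected; level-change helpers have no callers here.
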(event `self.ReceiveBeginPlay`
  (bind _asvrpawn (cast `/Game/Game/Benji/VRPawn` (`GameplayStatics.GetPlayerPawn` 0)))
  (bind _output_get (set `self.VRPawn` _asvrpawn))
  (set `self.Black Screen` (`/Game/Game/Benji/VRPawn.BlackScreen` _output_get))
  (set `self.White Screen` (`/Game/Game/Benji/VRPawn.WhiteScreen` _output_get))
  (bind _returnvalue (`GameplayStatics.GetActorOfClass` "/Game/Game/Ludo/BP_SplinePerso.BP_SplinePerso_C"))
  (set `self.BP_Spline` _returnvalue))

(event `self.ReceiveTick`
  (params (DeltaSeconds :type "Float (single-precision)"))
  (`KismetSystemLibrary.PrintString` (`KismetStringLibrary.Conv_DoubleToString` (`SplineComponent.GetSplineLength` (`/Game/Game/Ludo/BP_SplinePerso.Spline` (`self.BP_Spline`)))))
  (if (`self.IsMoving`)
    ;[1 1 1] Vérification de la fin de boucle
    (if (`self.IsLoopEnd`)
      (if (`KismetStringLibrary.EqualEqual_StrStr` (`self.LevelName`) "LevelFinal")
        (set `self.IsMoving` false)
        (else
          (set `self.IsAlreadyPause` false)
          (set `self.IsLoopEnd` false)
          (goto _label_2 :!via `Reset`)))
      (else
        (`|ExecutionSequence`
          (:`then_0`
            (if (`KismetStringLibrary.EqualEqual_StrStr` (`self.LevelName`) "LevelTestCigale")
              (bind _bool (`self.TestPosition` 2.0 50.0)) ; La valeur DiviseurDistance ne peut être égale à 0 (sinon ça crée une division par 0 et de potentielles erreurs)\nLa valeur MargeErreur représente la distance autorisée d'erreur
              (if (or _bool (stale _bool_2) (stale _bool_3)) :!label _label
                (`/Engine/EditorBlueprintResources/StandardMacros.DoOnce` false :!label _label_2
                  (:`Completed`
                    (`self.Stop Move`)
                    (`KismetSystemLibrary.Delay` 2.0)
                    (set `self.ConteurTemps` (+ (`self.ConteurTemps`) 2.0))
                    (`|ExecutionSequence`
                      (:`then_0`
                        (`self.PlayMove`))
                      (:`then_1`
                        (`self.Deplacement`)
                        (set `self.IsAlreadyPause` true)))))
                (else
                  (`self.Deplacement`)))))
          (:`then_1`
            (if (`KismetStringLibrary.EqualEqual_StrStr` (`self.LevelName`) "Map_VillageProvence")
              (bind _bool_2 (`self.TestPosition` 2.0 50.0))
              (goto _label)))
          (:`then_2`
            (if (`KismetStringLibrary.EqualEqual_StrStr` (`self.LevelName`) "VRTemplateMap")
              (bind _bool_3 (`self.TestPosition` 2.0 50.0))
              (goto _label))))))
    (else
      (set `self.ConteurTemps` (`GameplayStatics.GetTimeSeconds`)) ; Permet de recalculer le temps du jeu pour que la luciole puisse être situé au bon endroit sur la spline
    )))

(event `EndLevelTransition`
  (`/Game/Game/Yoann/BPW_BlackScreen.FadeInEvent` (`self.Black Screen`))
  (`KismetSystemLibrary.Delay` 1.1)
  (`GameplayStatics.OpenLevel` "VRTemplateMap"))

(fn `ChangementLevel`
  (bind _levellist (`/Game/Game/Benji/GI_TP.LevelList` (`self.GameInstance`)))
  (`/Engine/EditorBlueprintResources/StandardMacros.DoOnce` false :!label _label
    (:`Completed`
      (bind _returnvalue (`GameplayStatics.GetCurrentLevelName` true))
      (`GameplayStatics.OpenLevel` (`KismetStringLibrary.Conv_StringToName` (`|GetArrayItem` _levellist (+ (`KismetArrayLibrary.Array_Find` _levellist _returnvalue) 1))))
      (goto _label :!via `Reset`))))

(fn `Deplacement`
  (bind _spline (`/Game/Game/Ludo/BP_SplinePerso.Spline` (`self.BP_Spline`)))
  (bind _returnvalue (`SplineComponent.GetSplineLength` _spline))
  (bind _returnvalue_2 (mod (* (- (`GameplayStatics.GetTimeSeconds`) (`self.ConteurTemps`)) (`self.Speed`)) _returnvalue))
  (set `self.IsLoopEnd` (>= _returnvalue_2 (- _returnvalue 30.0)))
  (`SceneComponent.K2_SetWorldLocation` (`self.Plane`) (`SplineComponent.GetLocationAtDistanceAlongSpline` _spline _returnvalue_2 "World") false false))

(fn `Stop Move`
  (set `self.Speed` 0.0))

(fn `TestPosition`
  (params (DiviseurDistance :type "Float (double-precision)") (MargeErreur :type "Float (double-precision)"))
  (returns (Bool :type Boolean))
  (bind _spline (`/Game/Game/Ludo/BP_SplinePerso.Spline` (`self.BP_Spline`)))
  (return (and (== (`SplineComponent.GetLocationAtDistanceAlongSpline` _spline (/ (`SplineComponent.GetSplineLength` _spline) DiviseurDistance) "World") (`SceneComponent.K2_GetComponentLocation` (`self.Plane`)) :`ErrorTolerance` MargeErreur) (not (`self.IsAlreadyPause`)))))

(fn `UserConstructionScript`)