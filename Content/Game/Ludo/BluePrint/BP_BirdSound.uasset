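; BP_BirdSound is an actor in the Ludo game, apparently meant for timed ambient bird calls.
; On BeginPlay it runs a one-shot chain of three increasing delays, each followed by a play-sound call at the actor's location with no sound assigned.
; A disconnected four-step chain that references Bird_noise_Cue never runs, so the bird cue is not played by this graph.
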(event `self.ReceiveBeginPlay`
  (`KismetSystemLibrary.Delay` 10.0)
  (`GameplayStatics.PlaySoundAtLocation` null (`self.K2_GetActorLocation` self) (struct) 1.0 1.0 0.0 null null null null)
  (`KismetSystemLibrary.Delay` 25.0)
  (`GameplayStatics.PlaySoundAtLocation` null (`self.K2_GetActorLocation` self) (struct) 1.0 1.0 0.0 null null null null)
  (`KismetSystemLibrary.Delay` 40.0)
  (`GameplayStatics.PlaySoundAtLocation` null (`self.K2_GetActorLocation` self) (struct) 1.0 1.0 0.0 null null null null))

(fn `UserConstructionScript`)