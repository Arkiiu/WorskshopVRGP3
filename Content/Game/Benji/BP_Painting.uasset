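; Painting actor that displays one of the Provence, Lavande or Paris paintings depending on the current level.
; On BeginPlay it reads LevelIndex from the GI_TP game instance and hides the components that do not match, or all three for index 3 and any unhandled index.
; It also prints the hidden components' Visible state to the screen as debug output.
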(event `self.ReceiveBeginPlay`
  (bind _painting_paris (`self.Painting_Paris`))
  (bind _painting_provence (`self.Painting_Provence`))
  (bind _painting_lavande (`self.Painting_Lavande`))
  (bind _painting_provence_2 (`self.Painting_Provence`))
  (bind _painting_lavande_2 (`self.Painting_Lavande`))
  (bind _painting_paris_2 (`self.Painting_Paris`))
  (bind _painting_lavande_3 (`self.Painting_Lavande`))
  (bind _painting_paris_3 (`self.Painting_Paris`))
  (bind _painting_provence_3 (`self.Painting_Provence`))
  (bind _asgi_tp (cast `/Game/Game/Benji/GI_TP` (`GameplayStatics.GetGameInstance`)))
  (switch `int` (`/Game/Game/Benji/GI_TP.LevelIndex` _asgi_tp) ; En fonction de l'index du niveau actuel il effectue les tâche correspondantes
    (:`Default`
      (`SceneComponent.SetVisibility` _painting_provence_3 false false :!label _label)
      (`SceneComponent.SetVisibility` _painting_lavande false false)
      (`SceneComponent.SetVisibility` _painting_paris false false)
      (`KismetSystemLibrary.PrintString` (`KismetStringLibrary.Conv_BoolToString` (`SceneComponent.bVisible` _painting_provence_3)) true true (struct :`R` 1.0 :`B` 0.018385 :`A` 1.0))
      (`KismetSystemLibrary.PrintString` (`KismetStringLibrary.Conv_BoolToString` (`SceneComponent.bVisible` _painting_lavande)) true true (struct :`R` 0.079696 :`G` 1.0 :`A` 1.0))
      (`KismetSystemLibrary.PrintString` (`KismetStringLibrary.Conv_BoolToString` (`SceneComponent.bVisible` _painting_paris))))
    (:`0`
      (`SceneComponent.SetVisibility` _painting_lavande_3 false false)
      (`SceneComponent.SetVisibility` _painting_paris_3 false false)
      (`KismetSystemLibrary.PrintString` (`KismetStringLibrary.Conv_BoolToString` (`SceneComponent.bVisible` _painting_lavande_3)) true true (struct :`R` 1.0 :`B` 0.018385 :`A` 1.0))
      (`KismetSystemLibrary.PrintString` (`KismetStringLibrary.Conv_BoolToString` (`SceneComponent.bVisible` _painting_paris_3)) true true (struct :`R` 0.079696 :`G` 1.0 :`A` 1.0)))
    (:`1`
      (`SceneComponent.SetVisibility` _painting_provence false false)
      (`SceneComponent.SetVisibility` _painting_paris_2 false false)
      (`KismetSystemLibrary.PrintString` (`KismetStringLibrary.Conv_BoolToString` (`SceneComponent.bVisible` _painting_provence)) true true (struct :`R` 1.0 :`B` 0.018385 :`A` 1.0))
      (`KismetSystemLibrary.PrintString` (`KismetStringLibrary.Conv_BoolToString` (`SceneComponent.bVisible` _painting_paris_2)) true true (struct :`R` 0.079696 :`G` 1.0 :`A` 1.0)))
    (:`2`
      (`SceneComponent.SetVisibility` _painting_provence_2 false false)
      (`SceneComponent.SetVisibility` _painting_lavande_2 false false)
      (`KismetSystemLibrary.PrintString` (`KismetStringLibrary.Conv_BoolToString` (`SceneComponent.bVisible` _painting_provence_2)) true true (struct :`R` 1.0 :`B` 0.018385 :`A` 1.0))
      (`KismetSystemLibrary.PrintString` (`KismetStringLibrary.Conv_BoolToString` (`SceneComponent.bVisible` _painting_lavande_2)) true true (struct :`R` 0.079696 :`G` 1.0 :`A` 1.0)))
    (:`3`
      (goto _label))))

(event `self.ReceiveTick`
  (params (DeltaSeconds :type "Float (single-precision)")))

(fn `UserConstructionScript`)