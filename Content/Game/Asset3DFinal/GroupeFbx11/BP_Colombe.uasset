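; BP_Colombe is a dove actor that drives erratic motion through random spline turns and smoothed mesh rotation.
; A self-repeating event waits a random few seconds, then yaws the Spline by a random amount up to a quarter turn either way.
; Each Tick eases StaticMesh1's yaw toward a Z-axis rotation built from the Sphere-to-StaticMesh offset.
; StaticMesh's position lerp toward Sphere has zero alpha, so it stays put.
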(event `Rotation`
  (bind _spline (`self.Spline`))
  (bind (_returnvalue_roll _returnvalue_pitch _returnvalue_yaw) (`KismetMathLibrary.BreakRotator` (`SceneComponent.K2_GetComponentRotation` _spline)))
  (`KismetSystemLibrary.Delay` (`KismetMathLibrary.RandomFloatInRange` 1.0 4.0))
  (`SceneComponent.K2_SetWorldRotation` _spline (`KismetMathLibrary.MakeRotator` _returnvalue_roll _returnvalue_pitch (+ _returnvalue_yaw (`KismetMathLibrary.RandomFloatInRange` -90.0 90.0))) false false)
  (`self.Rotation`))

(event `self.ReceiveBeginPlay`
  (`self.Rotation`))

(event `self.ReceiveTick`
  (params (DeltaSeconds :type "Float (single-precision)"))
  (bind _staticmesh1 (`self.StaticMesh1`))
  (bind _returnvalue (`SceneComponent.K2_GetComponentLocation` (`self.Sphere`)))
  (bind _returnvalue_2 (`SceneComponent.K2_GetComponentLocation` (`self.StaticMesh`)))
  (bind (_returnvalue_roll _returnvalue_pitch _returnvalue_yaw) (`KismetMathLibrary.BreakRotator` (`SceneComponent.K2_GetComponentRotation` _staticmesh1)))
  (bind (_returnvalue_roll_2 _returnvalue_pitch_2 _returnvalue_yaw_2) (`KismetMathLibrary.BreakRotator` (`KismetMathLibrary.MakeRotFromZ` (- _returnvalue_2 _returnvalue))))
  (`SceneComponent.K2_SetWorldLocation` (`self.StaticMesh`) (`KismetMathLibrary.VLerp` _returnvalue_2 _returnvalue) false false)
  (`SceneComponent.K2_SetWorldRotation` _staticmesh1 (`KismetMathLibrary.MakeRotator` _returnvalue_roll _returnvalue_pitch (`KismetMathLibrary.Lerp` _returnvalue_yaw _returnvalue_yaw_2 0.05)) false false))

(fn `UserConstructionScript`)