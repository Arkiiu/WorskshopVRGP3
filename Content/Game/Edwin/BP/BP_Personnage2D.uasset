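; BP_Personnage2D is an actor whose Cube component travels on a loop along a spline in the level.
; On BeginPlay it finds and caches the BP_splinePersonnage2D actor, then starts a Timeline.
; Each update multiplies the Timeline alpha by the spline length and sets the Cube's world location at that distance, without sweeping.
; When the Timeline finishes, it restarts from the beginning after a zero-second Delay.
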(event `self.ReceiveBeginPlay`
  (bind _spline (`/Game/Game/Edwin/BP/BP_splinePersonnage2D.Spline` (`self.spline personnage`)))
  (bind _returnvalue (`GameplayStatics.GetActorOfClass` "/Game/Game/Edwin/BP/BP_splinePersonnage2D.BP_splinePersonnage2D_C"))
  (set `self.spline personnage` _returnvalue)
  (bind (_direction _alpha) (`Timeline|Timeline` :!label _label)
    (:`Update`
      (`SceneComponent.K2_SetWorldLocation` (`self.Cube`) (`SplineComponent.GetLocationAtDistanceAlongSpline` _spline (* _alpha (`SplineComponent.GetSplineLength` _spline)) "World") false false))
    (:`Finished`
      (`KismetSystemLibrary.Delay` 0.0)
      (goto _label :!via `PlayFromStart`))))

(fn `UserConstructionScript`)